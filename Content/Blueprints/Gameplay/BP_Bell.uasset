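; Bell actor for the second minigame that the player activates by its bell number.
; ActivateBell plays the bell's sound at its location, then reports BellNumber to GM_MiniGame2.
; If the game mode confirms success, it plays a win sound, shows the WBP_WinBell widget and returns to L_Intro after five seconds.
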(event EventBeginPlay)

(event Collision|EventActorBeginOverlap
  (params (OtherActor :type Actor%20Object%20Reference)))

(event EventTick
  (params (DeltaSeconds :type Float%20%28single-precision%29)))

(event EventActivateBell
  (params (BellNum :type Integer))
  (Audio|PlaySoundatLocation (Variables|Default|GetSound) (Transformation|GetActorLocation) "0, 0, 0" 1.0 1.0 0.0 0 0 0 0)
  (bind _asgm_mini_game_2 (Utilities|Casting|CastToGM_MiniGame2 (Game|GetGameMode)))
  (bind _win_ (Default|NotifierbellActivate _asgm_mini_game_2 (Variables|Default|GetBellNumber)))
  (if _win_
    (Audio|PlaySound2D "/Game/SFX/Bell/WinBell_Cue.WinBell_Cue" 1.0 1.0 0.0 0 0)
    (bind _returnvalue (UserInterface|CreateWidget "/Game/Blueprints/Widgets/WBP_WinBell.WBP_WinBell_C"))
    (bind _output_get (Variables|Default|SetNewVar_0 _returnvalue))
    (UserInterface|Viewport|AddtoViewport _output_get 0)
    (Utilities|FlowControl|Delay 5.0)
    (Game|OpenLevel(byObjectReference) "/Game/Maps/L_Intro.L_Intro")))

(fn ConstructionScript)