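; BP_Board is the game board: it holds the ordered Cells path, looks up cells by number and wraps movement indices around it.
; Two extension cell sets start hidden; ChangeBoard increments GI_Loop's board number, then reveals the matching set and splices it into Cells at a hard-coded index.
; GI_Loop's cell index is bumped for cells inserted before it.
; InitBoard re-enters that switch on BeginPlay, reapplying only the current stage.
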(event Custom|InitBoard
  (bind _as_gi_loop (Variables|Default|GetAs%20GI%20Loop))
  (bind _as_gi_loop_2 (Variables|Default|GetAs%20GI%20Loop))
  (switch int (stale Custom|ChangeBoard _output_get)
    (:0
      ;[0.15 0.15 0.15 0.5] pas de extension
      (Development|PrintString "bug"))
    (:1
      (Audio|PlaySound2D "/Game/SFX/SFX_MagicalTwinkles.SFX_MagicalTwinkles" 0.5 1.0 0.0 0 0 false)
      (Variables|Default|SetIndexToAdd 2)
      (for _array_element (Variables|Default|GetExtension1)
        (Rendering|SetActorHiddenInGame _array_element false))
      (for _array_element_2 (Variables|Default|GetExtension1)
        (Utilities|Array|Insert (Variables|Default|GetCells) _array_element_2 (Variables|Default|GetIndexToAdd))
        (Variables|Default|SetIndexToAdd (+ (Variables|Default|GetIndexToAdd) 1))
        (if (> (Variables|/Game/Blueprints/Global/GI_Loop.GI_Loop_C|GetCellNumber _as_gi_loop) (Variables|Default|GetIndexToAdd))
          (Default|AddIndexwhenChangeBoard _as_gi_loop))))
    (:2
      (Audio|PlaySound2D "/Game/SFX/SFX_MagicalTwinkles.SFX_MagicalTwinkles" 0.5 1.0 0.0 0 0 false)
      (Variables|Default|SetIndexToAdd 16)
      (for _array_element_3 (Variables|Default|GetExtension2)
        (Rendering|SetActorHiddenInGame _array_element_3 false))
      ;[0.15 0.15 0.15 0.5] Pour éviter de sauter la premiere case de la deuxieme extension (je sais pas d'ou provient le bug)
      (Variables|Default|SetIndexToAdd (+ (Variables|Default|GetIndexToAdd) 1))
      (for _array_element_4 (Variables|Default|GetExtension2)
        (Utilities|Array|Insert (Variables|Default|GetCells) _array_element_4 (Variables|Default|GetIndexToAdd))
        (Variables|Default|SetIndexToAdd (+ (Variables|Default|GetIndexToAdd) 1))
        (if (> (Variables|/Game/Blueprints/Global/GI_Loop.GI_Loop_C|GetCellNumber _as_gi_loop_2) (Variables|Default|GetIndexToAdd))
          (Default|AddIndexwhenChangeBoard _as_gi_loop_2))))))

(event Custom|ChangeBoard
  (bind _as_gi_loop (Variables|Default|GetAs%20GI%20Loop))
  (bind _as_gi_loop_2 (Variables|Default|GetAs%20GI%20Loop))
  (bind _as_gi_loop_3 (Variables|Default|GetAs%20GI%20Loop))
  (bind _output_get (Variables|/Game/Blueprints/Global/GI_Loop.GI_Loop_C|SetChangeBoardNumber _as_gi_loop_2 (+ (Variables|/Game/Blueprints/Global/GI_Loop.GI_Loop_C|GetChangeBoardNumber _as_gi_loop_2) 1)))
  (switch int _output_get
    (:0
      ;[0.15 0.15 0.15 0.5] pas de extension
      (Development|PrintString "bug"))
    (:1
      (Audio|PlaySound2D "/Game/SFX/SFX_MagicalTwinkles.SFX_MagicalTwinkles" 0.5 1.0 0.0 0 0 false)
      (Variables|Default|SetIndexToAdd 2)
      (for _array_element (Variables|Default|GetExtension1)
        (Rendering|SetActorHiddenInGame _array_element false))
      (for _array_element_2 (Variables|Default|GetExtension1)
        (Utilities|Array|Insert (Variables|Default|GetCells) _array_element_2 (Variables|Default|GetIndexToAdd))
        (Variables|Default|SetIndexToAdd (+ (Variables|Default|GetIndexToAdd) 1))
        (if (> (Variables|/Game/Blueprints/Global/GI_Loop.GI_Loop_C|GetCellNumber _as_gi_loop) (Variables|Default|GetIndexToAdd))
          (Default|AddIndexwhenChangeBoard _as_gi_loop))))
    (:2
      (Audio|PlaySound2D "/Game/SFX/SFX_MagicalTwinkles.SFX_MagicalTwinkles" 0.5 1.0 0.0 0 0 false)
      (Variables|Default|SetIndexToAdd 16)
      (for _array_element_3 (Variables|Default|GetExtension2)
        (Rendering|SetActorHiddenInGame _array_element_3 false))
      ;[0.15 0.15 0.15 0.5] Pour éviter de sauter la premiere case de la deuxieme extension (je sais pas d'ou provient le bug)
      (Variables|Default|SetIndexToAdd (+ (Variables|Default|GetIndexToAdd) 1))
      (for _array_element_4 (Variables|Default|GetExtension2)
        (Utilities|Array|Insert (Variables|Default|GetCells) _array_element_4 (Variables|Default|GetIndexToAdd))
        (Variables|Default|SetIndexToAdd (+ (Variables|Default|GetIndexToAdd) 1))
        (if (> (Variables|/Game/Blueprints/Global/GI_Loop.GI_Loop_C|GetCellNumber _as_gi_loop_3) (Variables|Default|GetIndexToAdd))
          (Default|AddIndexwhenChangeBoard _as_gi_loop_3))))))

(event EventBeginPlay
  (Utilities|FlowControl|Sequence
    (:then_0
      (bind _asgi_loop (Utilities|Casting|CastToGI_Loop (Game|GetGameInstance)))
      (Variables|Default|SetAs%20GI%20Loop _asgi_loop))
    (:then_1
      (for _array_element (Variables|Default|GetExtension1)
        (Rendering|SetActorHiddenInGame _array_element true)))
    (:then_2
      (for _array_element_2 (Variables|Default|GetExtension2)
        (Rendering|SetActorHiddenInGame _array_element_2 true)))
    (:then_3
      (CallFunction|InitBoard))))

(event EventTick
  (params (DeltaSeconds :type Float%20%28single-precision%29)))

(fn ConstructionScript)

(fn GetCellbyNumber
  (params (Number :type Integer))
  (return (Utilities|Array|Get(acopy) (Variables|Default|GetCells) Number)))

(fn GetNextCelltoMove
  (params (CellNumber :type Integer))
  (return (Math|Integer|%(Integer) CellNumber (Utilities|Array|Length (Variables|Default|GetCells)))))