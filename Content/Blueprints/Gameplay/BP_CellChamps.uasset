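; BP_CellChamps is a one-shot trigger that enables the thanks state on the cell dialogue actor.
; BeginPlay caches the GI_Loop game instance, whose DeactivateCellChamps flag guards the Activate event.
; The first Activate finds BP_DialogueCell by class, sets its ActivateThanks flag, then sets the guard.
; Because the guard lives on the game instance, the trigger stays spent across level loads.
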(event EventBeginPlay
  (|CallParentFunction)
  (bind _asgi_loop (Utilities|Casting|CastToGI_Loop (Game|GetGameInstance)))
  (Variables|Default|SetAs%20GI%20Loop _asgi_loop))

(event Collision|EventActorBeginOverlap
  (params (OtherActor :type Actor%20Object%20Reference))
  (|CallParentFunction OtherActor) ; This node is disabled and will not be called.\nDrag off pins to build functionality.
)

(event EventTick
  (params (DeltaSeconds :type Float%20%28single-precision%29))
  (|CallParentFunction DeltaSeconds) ; This node is disabled and will not be called.\nDrag off pins to build functionality.
)

(event EventActivate
  (params (Pawn :type CBP%20Pawn%20Object%20Reference))
  (if (not (Variables|/Game/Blueprints/Global/GI_Loop.GI_Loop_C|GetDeactivateCellChamps (Variables|Default|GetAs%20GI%20Loop)))
    (bind _returnvalue (Actor|GetActorOfClass "/Game/Blueprints/Gameplay/BP_DialogueCell.BP_DialogueCell_C"))
    (Variables|/Game/Blueprints/Gameplay/BP_DialogueCell.BP_DialogueCell_C|SetActivateThanks _returnvalue true)
    (Variables|/Game/Blueprints/Global/GI_Loop.GI_Loop_C|SetDeactivateCellChamps (Variables|Default|GetAs%20GI%20Loop) true)))

(fn ConstructionScript
  (|CallParentFunction))