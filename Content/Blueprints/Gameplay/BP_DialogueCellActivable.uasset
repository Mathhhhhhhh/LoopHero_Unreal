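; Activable cell that plays a row-based dialogue through the pawn's dialogue widget, with optional gameplay rewards.
; Activate shows the dialogue component's current row unless deactivated; the thanks option also refills GameInstance loop energy and disables further dialogue.
; Update advances rows until finished, then closes the widget and either changes the Board or, if flagged, activates a linked cell, disables itself and hides the LeVieux actor.
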(event EventBeginPlay
  (|CallParentFunction)
  (bind _returnvalue (Actor|GetActorOfClass "/Game/Blueprints/Gameplay/BP_Board.BP_Board_C"))
  (Variables|Default|SetBoard _returnvalue))

(event Collision|EventActorBeginOverlap
  (params (OtherActor :type Actor%20Object%20Reference))
  (|CallParentFunction OtherActor) ; This node is disabled and will not be called.\nDrag off pins to build functionality.
)

(event EventTick
  (params (DeltaSeconds :type Float%20%28single-precision%29))
  (|CallParentFunction DeltaSeconds) ; This node is disabled and will not be called.\nDrag off pins to build functionality.
)

(event EventActivate
  (params (Pawn :type CBP%20Pawn%20Object%20Reference))
  (bind _bpc_dialoguecomponent (Variables|Default|GetBPC_DialogueComponent))
  (bind _gi_loop (Variables|/Game/Blueprints/Gameplay/CBP_Pawn.CBP_Pawn_C|GetGI_Loop Pawn))
  (bind _wbp_dialogue (Variables|/Game/Blueprints/Gameplay/CBP_Pawn.CBP_Pawn_C|GetWBP_Dialogue Pawn))
  (if (not (Variables|Default|GetDeactivateDialogue))
    (Default|GetCurrentDialogueRowData _bpc_dialoguecomponent)
    (bind _charactername (Default|GetCharacterfromCurrentRow _bpc_dialoguecomponent))
    (bind _dialoguelong (Default|GetDialogueLongfromCurrentRow _bpc_dialoguecomponent))
    (Default|UpdateDialogue _wbp_dialogue _charactername _dialoguelong)
    (Default|StartDialogue _wbp_dialogue)
    (if (Variables|Default|GetActivateThanks)
      (Default|Thanks (Variables|Default|GetBPC_DialogueComponent))
      (Variables|/Game/Blueprints/Global/GI_Loop.GI_Loop_C|SetEnergy _gi_loop (Variables|/Game/Blueprints/Global/GI_Loop.GI_Loop_C|GetMaxEnergy _gi_loop))
      (Variables|Default|SetDeactivateDialogue true))))

(event EventUpdate
  (params (Pawn :type CBP%20Pawn%20Object%20Reference))
  (bind _bpc_dialoguecomponent (Variables|Default|GetBPC_DialogueComponent))
  (bind _wbp_dialogue (Variables|/Game/Blueprints/Gameplay/CBP_Pawn.CBP_Pawn_C|GetWBP_Dialogue Pawn))
  (bind _activablecell (Variables|Default|GetActivableCell))
  (bind _isfinished_ (Default|IsDialogueFinished _bpc_dialoguecomponent))
  (if _isfinished_
    (Default|ExitDialogue _wbp_dialogue)
    (if (Variables|Default|GetUnlockBoard)
      (Default|ChangeBoard (Variables|Default|GetBoard))
      (elif (Variables|Default|GetActivateSomething)
        (Variables|/Game/Blueprints/Gameplay/BP_UnlockBoardCell.BP_UnlockBoardCell_C|SetIsActive? _activablecell true)
        (Default|ActivateParticles _activablecell)
        (Variables|Default|SetDeactivateDialogue true)
        (bind _returnvalue (Actor|GetActorOfClass "/Game/Blueprints/Dialogues/LeVieux_Blueprint.LeVieux_Blueprint_C"))
        (Rendering|SetActorHiddenInGame _returnvalue true)))
    (else
      (Default|ReadNextRow _bpc_dialoguecomponent)
      (Default|GetCurrentDialogueRowData _bpc_dialoguecomponent)
      (bind _charactername (Default|GetCharacterfromCurrentRow _bpc_dialoguecomponent))
      (bind _dialoguelong (Default|GetDialogueLongfromCurrentRow _bpc_dialoguecomponent))
      (Default|UpdateDialogue _wbp_dialogue _charactername _dialoguelong))))

(fn ConstructionScript
  (|CallParentFunction))