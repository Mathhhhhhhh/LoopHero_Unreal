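; BP_DialogueCellMiniGame2 is a cell actor that launches the second minigame level, L_MiniGame2, when activated.
; On BeginPlay it caches the BP_Board actor and the GI_Loop game instance.
; Activate checks that the game instance's DeactivateMG2 flag is off and ActivateThanksDial is on, then opens the level after a short delay.
; It then sets DeactivateMG2 on the game instance to block later launches.
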(event EventBeginPlay
  (|CallParentFunction)
  (Utilities|FlowControl|Sequence
    (:then_0
      (bind _returnvalue (Actor|GetActorOfClass "/Game/Blueprints/Gameplay/BP_Board.BP_Board_C"))
      (Variables|Default|SetBoard _returnvalue))
    (:then_1
      (bind _asgi_loop (Utilities|Casting|CastToGI_Loop (Game|GetGameInstance)))
      (Variables|Default|SetAs%20GI%20Loop _asgi_loop))))

(event Collision|EventActorBeginOverlap
  (params (OtherActor :type Actor%20Object%20Reference))
  (|CallParentFunction OtherActor) ; This node is disabled and will not be called.\nDrag off pins to build functionality.
)

(event EventTick
  (params (DeltaSeconds :type Float%20%28single-precision%29))
  (|CallParentFunction DeltaSeconds) ; This node is disabled and will not be called.\nDrag off pins to build functionality.
)

(event EventActivate
  (params (Pawn :type CBP%20Pawn%20Object%20Reference))
  (if (not (Variables|/Game/Blueprints/Global/GI_Loop.GI_Loop_C|GetDeactivateMG2 (Variables|Default|GetAs%20GI%20Loop)))
    (if (Variables|/Game/Blueprints/Global/GI_Loop.GI_Loop_C|GetActivateThanksDial (Variables|Default|GetAs%20GI%20Loop))
      (Utilities|FlowControl|Delay 0.2)
      (Game|OpenLevel(byObjectReference) "/Game/Maps/L_MiniGame2.L_MiniGame2")
      (Variables|/Game/Blueprints/Global/GI_Loop.GI_Loop_C|SetDeactivateMG2 (Variables|Default|GetAs%20GI%20Loop) true))))

(fn ConstructionScript
  (|CallParentFunction))