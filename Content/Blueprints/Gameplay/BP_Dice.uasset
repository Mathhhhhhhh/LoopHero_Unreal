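; Dice actor that rolls a random step count to move a pawn at a cost in energy.
; On BeginPlay it caches the GI_Loop game instance and adds a WBP_Dice widget to the viewport, passing itself as that widget's Dice reference.
; RollTheDice picks an integer between the min and max dice values, passes it to the pawn's TryMoving, then spends a fixed amount of energy through GI_Loop.
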(event EventBeginPlay
  (Utilities|FlowControl|Sequence
    (:then_0
      (bind _asgi_loop (Utilities|Casting|CastToGI_Loop (Game|GetGameInstance)))
      (Variables|Default|SetAs%20GI%20Loop _asgi_loop))
    (:then_1
      (bind _returnvalue (UserInterface|CreateWidget "/Game/Blueprints/Widgets/WBP_Dice.WBP_Dice_C"))
      (Variables|/Game/Blueprints/Widgets/WBP_Dice.WBP_Dice_C|SetDice _returnvalue self)
      (Variables|Default|SetWidgetDice _returnvalue)
      (UserInterface|Viewport|AddtoViewport _returnvalue 0))))

(event Collision|EventActorBeginOverlap
  (params (OtherActor :type Actor%20Object%20Reference)))

(event EventTick
  (params (DeltaSeconds :type Float%20%28single-precision%29)))

(fn ConstructionScript)

(fn RolltheDice
  (bind _output_get (Variables|Default|SetValue (Math|Random|RandomIntegerinRange (Variables|Default|GetMinDiceValue) (Variables|Default|GetMaxDiceValue))))
  (Default|TryMoving (Variables|Default|GetPawn) _output_get)
  (Default|UseEnergy (Variables|Default|GetAs%20GI%20Loop) 2.0))