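; Board cell that, when activated, switches the game board, going by its name as an unlock cell.
; On BeginPlay it finds and caches the BP_Board actor in the level.
; If the cell is active, Activate calls ChangeBoard on that board and snaps its Camera1 to Camera2's location and rotation.
; A separate ActivateParticles event turns on the light insects effect without resetting it.
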(event Custom|ActivateParticles
  (params (Pawn :type CBP%20Pawn%20Object%20Reference))
  (Components|Activation|Activate (Variables|Default|GetPfx_LightInsects) false))

(event EventBeginPlay
  (|CallParentFunction)
  (bind _returnvalue (Actor|GetActorOfClass "/Game/Blueprints/Gameplay/BP_Board.BP_Board_C"))
  (Variables|Default|SetBoard _returnvalue))

(event Collision|EventActorBeginOverlap
  (params (OtherActor :type Actor%20Object%20Reference))
  (|CallParentFunction OtherActor) ; This node is disabled and will not be called.\nDrag off pins to build functionality.
)

(event EventTick
  (params (DeltaSeconds :type Float%20%28single-precision%29))
  (|CallParentFunction DeltaSeconds) ; This node is disabled and will not be called.\nDrag off pins to build functionality.
)

(event EventActivate
  (params (Pawn :type CBP%20Pawn%20Object%20Reference))
  (bind _board (Variables|Default|GetBoard))
  (bind _camera2 (Variables|/Game/Blueprints/Gameplay/BP_Board.BP_Board_C|GetCamera2 _board))
  (if (Variables|Default|GetIsActive?)
    (Default|ChangeBoard (Variables|Default|GetBoard))
    (Transformation|SetActorLocationAndRotation (Variables|/Game/Blueprints/Gameplay/BP_Board.BP_Board_C|GetCamera1 _board) (Transformation|GetActorLocation _camera2) (Transformation|GetActorRotation _camera2))))

(fn ConstructionScript
  (|CallParentFunction))