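; CBP_Pawn is the player pawn for a dice board game, placed on the board cell whose number is stored in the GI_Loop game instance.
; On BeginPlay it snaps to that cell and creates the dialogue UI, linking it to the dice widget and itself.
; TryMoving asks the Board for the destination, saves it to the game instance, teleports slightly above the cell and activates it.
; UpdateCell forwards an update message to the current cell.
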(event EventBeginPlay
  (bind _asgi_loop (Utilities|Casting|CastToGI_Loop (Game|GetGameInstance)))
  (Variables|Default|SetGI_Loop _asgi_loop)
  (CallFunction|MovetoCell)
  (bind _returnvalue (UserInterface|CreateWidget "/Game/Blueprints/Widgets/WBP_DialogueUI.WBP_DialogueUI_C"))
  (bind _output_get (Variables|Default|SetWBP_Dialogue _returnvalue))
  (Variables|/Game/Blueprints/Widgets/WBP_DialogueUI.WBP_DialogueUI_C|SetWBP_Dice _output_get (Variables|/Game/Blueprints/Gameplay/BP_Dice.BP_Dice_C|GetWidgetDice (Variables|Default|GetDice)))
  (Variables|/Game/Blueprints/Widgets/WBP_DialogueUI.WBP_DialogueUI_C|SetPawn _output_get self)
  (UserInterface|Viewport|AddtoViewport _output_get 0))

(event Collision|EventActorBeginOverlap
  (params (OtherActor :type Actor%20Object%20Reference)))

(event EventTick
  (params (DeltaSeconds :type Float%20%28single-precision%29)))

(fn ConstructionScript)

(fn MovetoCell
  (bind _cell (Default|GetCellbyNumber (Variables|Default|GetBoard) (Variables|/Game/Blueprints/Global/GI_Loop.GI_Loop_C|GetCellNumber (Variables|Default|GetGI_Loop))))
  (Transformation|SetActorTransform (Math|Transform|MakeTransform (+ (.location (Transformation|GetActorTransform _cell)) "0.000000,0.000000,6.000000") (.rotation (Transformation|GetActorTransform _cell)) "1.000000,1.000000,1.000000")))

(fn TryMoving
  (params (Value :type Integer))
  (bind _gi_loop (Variables|Default|GetGI_Loop))
  (bind _cell (Default|GetNextCelltoMove (Variables|Default|GetBoard) (+ Value (Variables|/Game/Blueprints/Global/GI_Loop.GI_Loop_C|GetCellNumber _gi_loop))))
  (bind _output_get (Variables|/Game/Blueprints/Global/GI_Loop.GI_Loop_C|SetCellNumber _gi_loop _cell))
  (CallFunction|MovetoCell)
  (CallFunction|ActivateCell)
  (Development|PrintString (Utilities|String|ToString(Integer) _output_get)))

(fn ActivateCell
  (bind _cell (Default|GetCellbyNumber (Variables|Default|GetBoard) (Variables|/Game/Blueprints/Global/GI_Loop.GI_Loop_C|GetCellNumber (Variables|Default|GetGI_Loop))))
  (Class|BPIActivable|Activate(Message) _cell self))

(fn UpdateCell
  (bind _cell (Default|GetCellbyNumber (Variables|Default|GetBoard) (Variables|/Game/Blueprints/Global/GI_Loop.GI_Loop_C|GetCellNumber (Variables|Default|GetGI_Loop))))
  (Class|BPIActivable|Update(Message) _cell self))