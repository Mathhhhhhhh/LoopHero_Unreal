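; GI_Loop is a Game Instance, judging by its prefix, that holds a cell counter and an energy pool for a board-based game.
; AddIndexWhenChangeBoard increments CellNumber by one, by its name when the board changes.
; UseEnergy subtracts a given cost from Energy, or quits the game outright when Energy is lower than that cost.
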(event Custom|UseEnergy
  (params (Cost :type Float%20%28double-precision%29))
  (if (>= (Variables|Default|GetEnergy) Cost)
    (Variables|Default|SetEnergy (- (Variables|Default|GetEnergy) Cost))
    (else
      (Game|QuitGame 0 "Quit" false))))

(event Custom|AddIndexWhenChangeBoard
  (Variables|Default|SetCellNumber (+ (Variables|Default|GetCellNumber) 1)))