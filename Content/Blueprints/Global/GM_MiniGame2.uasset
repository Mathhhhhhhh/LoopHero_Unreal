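; Game mode for the second minigame, a puzzle where bells must be activated in a set order.
; On BeginPlay it has the player controller possess the minigame pawn, switches to game-only input and hides the cursor.
; NotifierbellActivate checks each bell against the next GoodSequence entry, recording matches and returning whether the sequence is complete.
; A wrong bell clears the progress and plays a losing sound.
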(event EventBeginPlay
  (bind _returnvalue (Game|GetPlayerController 0))
  (bind _ascbp_pawn_mini_game_2 (Utilities|Casting|CastToCBP_PawnMiniGame2 (Game|Player|GetPlayerPawn 0)))
  (Pawn|Possess _returnvalue _ascbp_pawn_mini_game_2)
  (Input|SetInputModeGameOnly _returnvalue false)
  (Variables|/Script/Engine.PlayerController|SetbShowMouseCursor _returnvalue false))

(fn ConstructionScript)

(fn NotifierbellActivate
  (params (BellNum :type Integer))
  (bind _output_get (Variables|Default|SetBell%20Num BellNum))
  (if (== _output_get (Utilities|Array|Get(acopy) (Variables|Default|GetGoodSequence) (Utilities|Array|Length (Variables|Default|GetCurrentSequence))))
    (Utilities|Array|Add (Variables|Default|GetCurrentSequence) (Variables|Default|GetBell%20Num))
    (return (== (Utilities|Array|Length (Variables|Default|GetGoodSequence)) (Utilities|Array|Length (Variables|Default|GetCurrentSequence))))
    (else
      (Utilities|Array|Clear (Variables|Default|GetCurrentSequence))
      (Audio|PlaySound2D "/Game/SFX/Bell/LoseBell_Cue.LoseBell_Cue" 1.0 1.0 0.0 0 0))))