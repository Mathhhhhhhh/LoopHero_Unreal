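; BP_LoopHero is a character that makes the player lose a minigame by getting too close.
; BeginPlay caches the player pawn as CBP_PawnMiniGame1, and Tick sets its Lose flag whenever its distance is within AttackRange.
; With CacheCache set, movement is deactivated then immediately reactivated, as the intended Delay is disconnected.
; A debug print of IsInAttackRange is also left unwired.
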(event EventBeginPlay
  (bind _charactermovement (Variables|Character|GetCharacterMovement))
  (Utilities|FlowControl|Sequence
    (:then_0
      (if (Variables|Default|GetCacheCache)
        (Components|Activation|Deactivate _charactermovement)
        (Components|Activation|Activate _charactermovement false)))
    (:then_1
      (bind _ascbp_pawn_mini_game_1 (Utilities|Casting|CastToCBP_PawnMiniGame1 (Game|Player|GetPlayerPawn 0)))
      (Variables|Default|SetBP_PawnMG1 _ascbp_pawn_mini_game_1))))

(event EventTick
  (params (DeltaSeconds :type Float%20%28single-precision%29))
  (bind _bp_pawnmg1 (Variables|Default|GetBP_PawnMG1))
  (if (<= (Transformation|GetDistanceTo _bp_pawnmg1) (Variables|Default|GetAttackRange))
    (Variables|/Game/Blueprints/Gameplay/CBP_PawnMiniGame1.CBP_PawnMiniGame1_C|SetLose _bp_pawnmg1 true)))

(fn ConstructionScript)